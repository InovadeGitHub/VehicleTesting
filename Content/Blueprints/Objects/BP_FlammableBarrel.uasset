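; BP_FlammableBarrel is an explosive barrel that detonates when a fast-moving vehicle hits it.
; A box overlap checks vehicle velocity, plays a hit sound, then triggers the blast once after a short random delay.
; The explosion spawns particles, fires an impulse, starts a camera shake, plays sound and later destroys the barrel.
; An Explode event triggers the same blast directly, bypassing the speed check and DoOnce guard.
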(event `self.Box.OnComponentBeginOverlap`
  (params (OverlappedComponent :type "PrimitiveComponent Object Reference") (OtherActor :type "Actor Object Reference") (OtherComp :type "PrimitiveComponent Object Reference") (OtherBodyIndex :type Integer) (bFromSweep :type Boolean) (SweepResult :type "HitResult Structure (by ref)"))
  ;[1 0.1042 0.1042] Overlap
  (bind _asbp_vehicle_base (cast `/Game/Vehicles/Player/BP_VehicleBase` OtherActor))
  (if (>= (`/Game/Vehicles/Player/BP_VehicleBase.Get Vehicle Velocity` _asbp_vehicle_base) 1500.0)
    (`GameplayStatics.PlaySoundAtLocation` "/Game/Audio/SoundEffects/Objects/HitSounds/MetalBarrel/CUE_MetalBarrel_Hit.CUE_MetalBarrel_Hit" (`self.K2_GetActorLocation`) (struct) 2.0 1.0 0.0 null null null)
    (`KismetSystemLibrary.Delay` (`KismetMathLibrary.RandomFloatInRange` 0.1 0.2))
    (`/Engine/EditorBlueprintResources/StandardMacros.DoOnce` false
      (:`Completed`
        (`GameplayStatics.SpawnEmitterAtLocation` "/Game/Environment/Effects/Explosion/P_Explosion_03.P_Explosion_03" (`self.K2_GetActorLocation`) :!label _label)
        (`RadialForceComponent.FireImpulse` (`self.Blast Force`))
        (`CameraShakeSourceComponent.Start` (`self.Camera Shake`))
        (`GameplayStatics.PlaySoundAtLocation` "/Game/Audio/SoundEffects/Objects/FlammableBarrel/Explosion/CUE_FlammableBarrelExplosion.CUE_FlammableBarrelExplosion" (`self.K2_GetActorLocation`) (struct) (`KismetMathLibrary.RandomFloatInRange` 1.0 2.0) 1.0 0.0 null null null)
        (`KismetSystemLibrary.Delay` 4.0)
        (`self.K2_DestroyActor`)))))

(event `Explode`
  ;[1 0.1042 0.1042] Overlap
  (goto _label))

(fn `UserConstructionScript`)