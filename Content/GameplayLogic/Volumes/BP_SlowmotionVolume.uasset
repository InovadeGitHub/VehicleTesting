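; Trigger volume that puts the game into slow motion while a BP_VehicleBase overlaps its box.
; A timeline, paced by BlendSpeed, blends global time dilation toward DesiredTimeDilation and drives post-process gamma and chromatic aberration.
; Entry also pushes a slow-motion sound mix, while exit reverses the timeline and clears all sound mix modifiers.
; A DoOnce flag gates triggering, and a Debug flag reveals the box in game.
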(event `self.Box.OnComponentBeginOverlap`
  (params (OverlappedComponent :type "PrimitiveComponent Object Reference") (OtherActor :type "Actor Object Reference") (OtherComp :type "PrimitiveComponent Object Reference") (OtherBodyIndex :type Integer) (bFromSweep :type Boolean) (SweepResult :type "HitResult Structure (by ref)"))
  (cast `/Game/Vehicles/Player/BP_VehicleBase` OtherActor)
  (if (`self.bDoOnce`)
    (`/Engine/EditorBlueprintResources/StandardMacros.DoOnce` false)
    (else
      (`TimelineComponent.SetPlayRate` (`self.TL_Slowmotion`) (/ 1.0 (`self.Blend Speed`)))
      (`GameplayStatics.PushSoundMixModifier` "/Game/Audio/SoundMixes/SMIX_Slowmotion.SMIX_Slowmotion")
      (bind (_direction _time_dilation _gamma _chromatic_aberration) (`Timeline|TL_Slowmotion` :!label _label)
        (:`Update`
          (`GameplayStatics.SetGlobalTimeDilation` (`KismetMathLibrary.Lerp` 1.0 (`self.Desired Time Dilation`) _time_dilation))
          (set `PostProcessComponent.Settings` (make `PostProcessSettings` :`ColorGamma` (`KismetMathLibrary.MakeVector4` 1.0 1.0 1.0 _gamma) :`SceneFringeIntensity` _chromatic_aberration) (`self.PostProcess`)))))))

(event `self.Box.OnComponentEndOverlap`
  (params (OverlappedComponent :type "PrimitiveComponent Object Reference") (OtherActor :type "Actor Object Reference") (OtherComp :type "PrimitiveComponent Object Reference") (OtherBodyIndex :type Integer))
  (cast `/Game/Vehicles/Player/BP_VehicleBase` OtherActor)
  (if (`self.bDoOnce`)
    (`/Engine/EditorBlueprintResources/StandardMacros.DoOnce` false
      (:`Completed`
        _)))
  (`TimelineComponent.Reverse` (`self.TL_Slowmotion`))
  (`GameplayStatics.ClearSoundMixModifiers`)
  (goto _label :!via `Reverse`))

(fn `UserConstructionScript`
  (if (`self.bDebug`)
    (`SceneComponent.SetHiddenInGame` (`self.Box`) false false)))