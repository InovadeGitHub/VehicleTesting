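; BP_IngameHUD is a vehicle HUD that draws the speed and gear readouts on screen while the owning BP_VehicleBase pawn's IsInCar flag is false.
; DrawHUD scales text position and size from a 1280x720 reference resolution, then draws the vehicle's speed and gear strings.
; The gear text switches between the vehicle's normal and reverse colors based on InReverseGear.
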(event `self.ReceiveDrawHUD`
  (params (SizeX :type Integer) (SizeY :type Integer))
  (bind _hudyratio (`self.HUDYRatio`))
  (bind _hudyratio_2 (`self.HUDYRatio`))
  (bind _asbp_vehicle_base (cast `/Game/Vehicles/Player/BP_VehicleBase` (`self.GetOwningPawn`)))
  (if (not (`/Game/Vehicles/Player/BP_VehicleBase.IsInCar` _asbp_vehicle_base))
    (`|ExecutionSequence`
      (:`then_0`
        (set `self.HUDXRatio` (/ (`KismetMathLibrary.Conv_IntToDouble` SizeX) 1280.0)))
      (:`then_1`
        (set `self.HUDYRatio` (/ (`KismetMathLibrary.Conv_IntToDouble` SizeY) 720.0)))
      (:`then_2`
        (bind _asbp_vehicle_base_2 (cast `/Game/Vehicles/Player/BP_VehicleBase` (`self.GetOwningPawn`)))
        (`self.DrawText` (`/Game/Vehicles/Player/BP_VehicleBase.Speed String` _asbp_vehicle_base_2) (struct :`R` 1.0 :`G` 1.0 :`B` 1.0 :`A` 1.0) (* 805.0 (`self.HUDXRatio`)) (* 455.0 _hudyratio_2) "/Engine/EngineFonts/RobotoDistanceField.RobotoDistanceField" (* 1.4 _hudyratio_2))
        (bind _asbp_vehicle_base_3 (cast `/Game/Vehicles/Player/BP_VehicleBase` (`self.GetOwningPawn`)))
        (`self.DrawText` (`KismetStringLibrary.Concat_StrStr` "Gear:" (`/Game/Vehicles/Player/BP_VehicleBase.Gear String` _asbp_vehicle_base_3)) (`KismetMathLibrary.SelectColor` (`/Game/Vehicles/Player/BP_VehicleBase.Gear Reverse Color` _asbp_vehicle_base_3) (`/Game/Vehicles/Player/BP_VehicleBase.Gear Color` _asbp_vehicle_base_3) (`/Game/Vehicles/Player/BP_VehicleBase.bInReverseGear` _asbp_vehicle_base_3)) (* 805.0 (`self.HUDXRatio`)) (* 500.0 _hudyratio) "/Engine/EngineFonts/RobotoDistanceField.RobotoDistanceField" (* 1.4 _hudyratio))))))

(fn `UserConstructionScript`)